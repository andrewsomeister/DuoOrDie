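; Zombie enemy character that roams slowly until it sees a character, then screams and chases it to attack.
; Roaming loops AIMoveTo to random navigable points with an idle bite montage.
; PawnSensing triggers a one-time timeline turn toward the target and scream, then a faster move-to and hit-montage loop.
; A failed move beyond a distance limit resets the DoOnce and returns to roaming.
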(event `Start Roaming`
  (set `CharacterMovementComponent.MaxWalkSpeed` 100.0 (`self.CharacterMovement`) :!label _label)
  (bind _randomlocation (`NavigationSystemV1.K2_GetRandomLocationInNavigableRadius` (`self.K2_GetActorLocation`) 1000.0 null null))
  (`|AIMoveTo` self _randomlocation null 70.0
    (:`OnSuccess`
      (`self.PlayAnimMontage` "/Game/EnemyAI/Animations/zombieIdleBite.zombieIdleBite"))
    (:`OnFail`
      _))
  (if (not (`self.SeesPlayer`))
    (`self.Start Roaming`)))

(event `self.ReceiveBeginPlay`
  (goto _label))

(event `self.PawnSensing.OnSeePawn`
  (params (Pawn :type "Pawn Object Reference"))
  (bind _ascharacter (cast `Character` Pawn))
  (set `self.MainCharacter` _ascharacter)
  (`self.Run After Player`)
  (set `self.SeesPlayer` true))

(event `Run To Player`
  (`|AIMoveTo` self (0.0 0.0 0.0) (`self.MainCharacter`) :!label _label_2
    (:`OnSuccess`
      (bind _returnvalue (`self.PlayAnimMontage` "/Game/EnemyAI/Animations/ZombieHit.ZombieHit" 1.7))
      (`KismetSystemLibrary.Delay` _returnvalue)
      (`self.Run To Player`))
    (:`OnFail`
      (if (> (`self.GetDistanceTo` (`self.MainCharacter`)) 3000.0)
        (`MovementComponent.StopMovementImmediately` (`self.CharacterMovement`))
        (`self.Start Roaming`)
        (set `self.SeesPlayer` false)
        (`self.PawnSenseReset`)
        (else
          (`self.Run To Player`))))))

(event `Run After Player`
  (`/Engine/EditorBlueprintResources/StandardMacros.DoOnce` false :!label _label_3
    (:`Completed`
      (`MovementComponent.StopMovementImmediately` (`self.CharacterMovement`))
      (`|ExecutionSequence`
        (:`then_0`
          (bind (_direction _newtrack_0) (`Timeline|Timeline` :!via `PlayFromStart`)
            (:`Update`
              (`self.K2_SetActorRotation` (`KismetMathLibrary.RLerp` (`self.K2_GetActorRotation`) (`KismetMathLibrary.FindLookAtRotation` (`self.K2_GetActorLocation`) (`self.K2_GetActorLocation` (`self.MainCharacter`))) _newtrack_0)))))
        (:`then_1`
          (bind _returnvalue (`self.PlayAnimMontage` "/Game/EnemyAI/Animations/ZombieScream.ZombieScream"))
          (`KismetSystemLibrary.Delay` _returnvalue)
          (set `CharacterMovementComponent.MaxWalkSpeed` 600.0 (`self.CharacterMovement`))
          (goto _label_2))))))

(event `PawnSenseReset`
  (set `CharacterMovementComponent.MaxWalkSpeed` 100.0 (`self.CharacterMovement`))
  (goto _label_3 :!via `Reset`))

(fn `UserConstructionScript`)