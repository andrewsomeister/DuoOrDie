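; BP_1Player2Collectible is a Level 1 pickup actor that a player character collects by touch.
; When a Correct_First_Person_Char overlaps TriggerZone, it plays a coin sound at its location and destroys itself.
; The IdNum check for player 2 is unwired, so any character of that class collects it.
; SpawnLocation sets a random X/Y position after an empty loop, but nothing here calls it.
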(event `self.ReceiveTick`
  (params (DeltaSeconds :type "Float (single-precision)")))

(event `self.TriggerZone.OnComponentBeginOverlap`
  (params (OverlappedComponent :type "PrimitiveComponent Object Reference") (OtherActor :type "Actor Object Reference") (OtherComp :type "PrimitiveComponent Object Reference") (OtherBodyIndex :type Integer) (bFromSweep :type Boolean) (SweepResult :type "HitResult Structure (by ref)"))
  (bind _ascorrect_first_person_char (cast `/Game/ConnorsManualUploads/Correct_First_Person_Char` OtherActor))
  (`GameplayStatics.PlaySoundAtLocation` "/Game/Maze/NintendoCoinPickup.NintendoCoinPickup" (`self.K2_GetActorLocation`) (struct) 1.0 1.0 0.0 null null null null)
  (`self.K2_DestroyActor`))

(fn `SpawnLocation`
  (for _ (range 5)
    _)
  (`self.K2_SetActorLocation` (`KismetMathLibrary.MakeVector` (`KismetMathLibrary.RandomFloatInRange` -7110.0 10600.0) (`KismetMathLibrary.RandomFloatInRange` -155000.0 1840.0))))

(fn `UserConstructionScript`)